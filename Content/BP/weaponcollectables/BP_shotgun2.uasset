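; BP_shotgun2 is a shotgun weapon actor, filed with weapon collectables, that fires a single BP_bullet per shot.
; CustomEvent_0 forwards a spawn transform to CustomEvent_1, which requires a valid ActorAttached on the Arkde character reference.
; It then spawns the bullet at that transform, an explosion emitter at the Arrow component and the shot sound at the actor.
; Disconnected leftovers include an Arrow-based fire call and mouse-driven rotation, neither of which runs.
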(event Custom|CustomEvent_0
  (params (SpawnTransform :type Transform))
  (CallFunction|CustomEvent1 SpawnTransform))

(event Custom|CustomEvent_1
  (params (SpawnTransform :type Transform))
  (bind _arrow (Variables|Default|GetArrow))
  (bind _returnvalue (Transformation|GetWorldTransform _arrow))
  (Variables|/Game/BP/Character/BP_ArkdeCharacter.BP_ArkdeCharacter_C|GetactorAttached (Variables|Default|GetAs%20BP%20Arkde%20Character)
    (:then
      (Game|SpawnActorfromClass "/Game/BP/weaponcollectables/BP_bullet.BP_bullet_C" SpawnTransform "Undefined" 0 0)
      (Effects|SpawnEmitteratLocation "/Game/StarterContent/Particles/P_ExplosionWeapon.P_ExplosionWeapon" (.location _returnvalue) (.rotation _returnvalue) (.scale _returnvalue))
      (Audio|SpawnSoundatLocation "/Game/BP/Sounds/shoot.shoot" (Transformation|GetActorLocation) "0, 0, 0" 5.0 1.0 0.0 0 0))
    (:else)))

(event EventBeginPlay
  (|CallParentFunction) ; This node is disabled and will not be called.\nDrag off pins to build functionality.
)

(event Collision|EventActorBeginOverlap
  (params (OtherActor :type Actor%20Object%20Reference))
  (|CallParentFunction OtherActor) ; This node is disabled and will not be called.\nDrag off pins to build functionality.
)

(event Input|ActionEvents|InputActionWeaponAction
  (params (Key :type Key%20Structure :default "None")))

(fn ConstructionScript
  (|CallParentFunction))