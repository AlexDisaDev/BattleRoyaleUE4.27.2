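; Bullet actor that damages Arkde characters on contact through the Gameplay Ability System and expires after a short server-set lifespan.
; Its sphere overlap ignores the instigator and, on authority only, applies the GE_FireboltDamage effect to the hit character's ability system.
; A valid hit then calls DestroyBulletClient, which spawns an explosion emitter, plays a 2D sound and destroys the actor.
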(event OnComponentBeginOverlap(SphereComponent)
  (params (OverlappedComponent :type Primitive%20Component%20Object%20Reference) (OtherActor :type Actor%20Object%20Reference) (OtherComp :type Primitive%20Component%20Object%20Reference) (OtherBodyIndex :type Integer) (bFromSweep :type Boolean) (SweepResult :type Hit%20Result%20Structure%20%28by%20ref%29))
  (if (!= OtherActor (Variables|Default|GetInstigator))
    (Networking|SwitchHasAuthority
      (:Authority
        (bind _asbp_arkde_character (Utilities|Casting|CastToBP_ArkdeCharacter OtherActor))
        (GameplayEffects|ApplyGameplayEffectToSelf :self (Ability|GetAbilitySystemComponent _asbp_arkde_character) :GameplayEffectClass "/Game/BP/Abilities/firebolt/GE_FireboltDamage.GE_FireboltDamage_C")
        (CallFunction|DestroyBulletClient)))))

(event Custom|DestroyBulletClient
  (Effects|SpawnEmitteratLocation "/Game/StarterContent/Particles/P_Explosion.P_Explosion" (Transformation|GetActorLocation))
  (Audio|PlaySound2D "/Game/StarterContent/Audio/Explosion02.Explosion02" 1.0 1.0 0.0 0 0)
  (Actor|DestroyActor))

(event EventBeginPlay
  (Networking|SwitchHasAuthority
    (:Authority
      (Actor|SetLifeSpan 3.0))))

(event Collision|EventActorBeginOverlap
  (params (OtherActor :type Actor%20Object%20Reference)))

(event EventTick
  (params (DeltaSeconds :type Float%20%28single-precision%29)))

(fn ConstructionScript)