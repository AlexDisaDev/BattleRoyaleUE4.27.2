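; BP_bullet is a short-lived projectile actor that scales itself down on spawn and leaves a smoke emitter trail every tick.
; Overlapping a BP_ArkdeCharacter other than its instigator sets that character's Hit flag, then passes through server and client custom events to destroy the bullet.
; Blood effect and GE_BulletDamage gameplay-effect logic exist but are disconnected, and the Tick authority switch has empty branches.
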(event OnComponentBeginOverlap(StaticMesh)
  (params (OverlappedComponent :type Primitive%20Component%20Object%20Reference) (OtherActor :type Actor%20Object%20Reference) (OtherComp :type Primitive%20Component%20Object%20Reference) (OtherBodyIndex :type Integer) (bFromSweep :type Boolean) (SweepResult :type Hit%20Result%20Structure%20%28by%20ref%29))
  (if (!= OtherActor (Game|GetInstigator))
    (bind _asbp_arkde_character (Utilities|Casting|CastToBP_ArkdeCharacter OtherActor))
    (Variables|/Game/BP/Character/BP_ArkdeCharacter.BP_ArkdeCharacter_C|Sethit _asbp_arkde_character true)
    (CallFunction|CEDamageBulletServer OtherActor)))

(event Custom|CE_DamageBulletClient
  (params (actor :type Actor%20Object%20Reference))
  (Actor|DestroyActor))

(event Custom|CE_DamageBulletServer
  (params (actor :type Actor%20Object%20Reference))
  (CallFunction|CEDamageBulletClient))

(event EventBeginPlay
  (Actor|SetLifeSpan 1e+01)
  (Transformation|SetActorScale3D "0.080000,0.050000,0.050000")
  (bind _asbp_arkde_character (Utilities|Casting|CastToBP_ArkdeCharacter (Game|GetPlayerCharacter 0)))
  (Variables|Default|SetAs%20BP%20Arkde%20Character _asbp_arkde_character))

(event Collision|EventActorBeginOverlap
  (params (OtherActor :type Actor%20Object%20Reference)))

(event EventTick
  (params (DeltaSeconds :type Float%20%28single-precision%29))
  (Networking|SwitchHasAuthority
    (:Authority
      _)
    (:Remote
      _))
  (Effects|SpawnEmitteratLocation "/Game/StarterContent/Particles/P_Smoke_bullet.P_Smoke_bullet" (Transformation|GetActorLocation) (Transformation|GetActorRotation) "0.200000,0.200000,0.200000"))

(fn ConstructionScript)