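; Shocking Grasp ability actor that drains health from a character it touches, living for a time derived from its range.
; On the server, a DoOnce lets only the first sphere overlap through, even if it is the instigator.
; If that actor is another BP_ArkdeCharacter, GAS effects damage it and heal the instigator.
; The particle component is then made visible, also only within that server branch.
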(event OnComponentBeginOverlap(SphereComponentH)
  (params (OverlappedComponent :type Primitive%20Component%20Object%20Reference) (OtherActor :type Actor%20Object%20Reference) (OtherComp :type Primitive%20Component%20Object%20Reference) (OtherBodyIndex :type Integer) (bFromSweep :type Boolean) (SweepResult :type Hit%20Result%20Structure%20%28by%20ref%29))
  (bind _returnvalue (Game|GetInstigator))
  (Networking|SwitchHasAuthority
    (:Authority
      (Utilities|FlowControl|DoOnce false
        (:Completed
          (if (!= OtherActor _returnvalue)
            (bind _asbp_arkde_character (Utilities|Casting|CastToBP_ArkdeCharacter OtherActor))
            (GameplayEffects|ApplyGameplayEffectToSelf :self (Class|ArkdeCMCharacter|GetAbilitySystemComponent _asbp_arkde_character) :GameplayEffectClass "/Game/BP/Abilities/ShockingGrasp/GE_ShockinggraspDamage.GE_ShockinggraspDamage_C")
            (GameplayEffects|ApplyGameplayEffectToSelf :self (Ability|GetAbilitySystemComponent _returnvalue) :GameplayEffectClass "/Game/BP/Abilities/ShockingGrasp/GE_Shockinggrasphealing.GE_Shockinggrasphealing_C")
            (Rendering|SetVisibility (Variables|Default|GetParticleSystemComponentH) true false)))))))

(event EventBeginPlay
  (Actor|SetLifeSpan (/ (Variables|Default|GetRangeH) 2e+03)))

(event Collision|EventActorBeginOverlap
  (params (OtherActor :type Actor%20Object%20Reference)))

(event EventTick
  (params (DeltaSeconds :type Float%20%28single-precision%29)))

(fn ConstructionScript)