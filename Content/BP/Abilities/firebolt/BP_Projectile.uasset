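; Firebolt ability projectile that explodes on hitting anything other than its instigator and briefly reveals struck characters on the minimap.
; On authority, a hit BP_ArkdeCharacter receives damage and burn Gameplay Effects and has its minimap pointer shown.
; DestroyEvent plays explosion effects, hides particles, disables collision, then after a delay hides that pointer and destroys the actor.
; Lifespan is set from the movement component's InitialSpeed value.
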(event OnComponentHit(SphereComponent)
  (params (HitComponent :type Primitive%20Component%20Object%20Reference) (OtherActor :type Actor%20Object%20Reference) (OtherComp :type Primitive%20Component%20Object%20Reference) (NormalImpulse :type Vector :default "0, 0, 0") (Hit :type Hit%20Result%20Structure%20%28by%20ref%29))
  (if (!= OtherActor (Game|GetInstigator))
    (Networking|SwitchHasAuthority
      (:Authority
        (bind _asbp_arkde_character (Utilities|Casting|CastToBP_ArkdeCharacter OtherActor)
          (:then
            (GameplayEffects|ApplyGameplayEffectToSelf :self (Class|ArkdeCMCharacter|GetAbilitySystemComponent _asbp_arkde_character) :GameplayEffectClass "/Game/BP/Abilities/firebolt/GE_FireboltDamage.GE_FireboltDamage_C")
            (GameplayEffects|ApplyGameplayEffectToSelf :self (Class|ArkdeCMCharacter|GetAbilitySystemComponent _asbp_arkde_character) :GameplayEffectClass "/Game/BP/Abilities/firebolt/GE_FirboltBurn.GE_FirboltBurn_C")
            (CallFunction|ShowEnemy _asbp_arkde_character))
          (:CastFailed
            _))
        (CallFunction|DestroyEvent (.ImpactPoint (Collision|BreakHitResult Hit)))))))

(event Custom|DestroyEvent
  (params (ImpactPoint :type Vector))
  ;[1 0.008526 0] destruccion del proyectil con sus sonidos y particulas
  (Utilities|IsValid self
    (:Is%20Valid
      (Audio|PlaySoundatLocation "/Game/StarterContent/Audio/Explosion01.Explosion01" ImpactPoint "0, 0, 0" 1.0 1.0 0.0 0 0 0)
      (Effects|SpawnEmitteratLocation "/Game/FXVarietyPack/Particles/P_ky_explosion_2.P_ky_explosion_2" ImpactPoint)
      (Utilities|IsValid self
        (:Is%20Valid
          (bind _particlesystemcomponent (Variables|Default|GetParticleSystemComponent)
            (:then
              (Rendering|SetVisibility _particlesystemcomponent false true)
              (bind _spherecomponent (Variables|Default|GetSphereComponent)
                (:then
                  (Collision|SetCollisionEnabled _spherecomponent "NoCollision")
                  (Utilities|FlowControl|Delay 6.0)
                  (CallFunction|EnemyDesapear (stale OnComponentHit(SphereComponent) _asbp_arkde_character))
                  (Actor|DestroyActor))
                (:else)))
            (:else)))))))

(event Custom|ShowEnemy
  (params (actor :type Actor%20Object%20Reference))
  (bind _returnvalue (Actor|GetComponentbyClass actor "/Game/BP/MinmapBigMap/AC_Pointerminimap.AC_Pointerminimap_C"))
  ;[0 1 0.01307] mostrar enemigo en el minimap si el proyectil lo impacta
  (Variables|/Game/BP/MinmapBigMap/AC_Pointerminimap.AC_Pointerminimap_C|SetIsVisible _returnvalue true)
  (Default|ReaddPointOfEnemy _returnvalue actor))

(event Custom|EnemyDesapear
  (params (actor :type Actor%20Object%20Reference))
  (bind _returnvalue (Actor|GetComponentbyClass actor "/Game/BP/MinmapBigMap/AC_Pointerminimap.AC_Pointerminimap_C"))
  ;[1 0.009454 0] desaparecer al enemigo del minimap
  (Utilities|IsValid actor
    (:Is%20Valid
      (Variables|/Game/BP/MinmapBigMap/AC_Pointerminimap.AC_Pointerminimap_C|SetIsVisible _returnvalue false)
      (Default|ReaddPointOfEnemy _returnvalue actor))))

(event EventBeginPlay
  (Actor|SetLifeSpan (Variables|/Script/Engine.ProjectileMovementComponent|GetInitialSpeed (Variables|Default|GetProjectileMovementComponent))))

(event Collision|EventActorBeginOverlap
  (params (OtherActor :type Actor%20Object%20Reference)))

(event EventTick
  (params (DeltaSeconds :type Float%20%28single-precision%29)))

(fn ConstructionScript)