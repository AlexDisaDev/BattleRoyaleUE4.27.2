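; BP_Storm is a battle royale-style shrinking safe zone that damages BP_ArkdeCharacters outside it.
; A server countdown triggers each phase, placing and revealing the zone once at a random location, then shrinking it by timeline by a random amount until scale reaches zero.
; Server overlap events apply the GE_StormDamage gameplay effect on exit and remove it on entry.
; The timeline-driven movement logic is disconnected and never runs.
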(event OnComponentBeginOverlap(Storm)
  (params (OverlappedComponent :type Primitive%20Component%20Object%20Reference) (OtherActor :type Actor%20Object%20Reference) (OtherComp :type Primitive%20Component%20Object%20Reference) (OtherBodyIndex :type Integer) (bFromSweep :type Boolean) (SweepResult :type Hit%20Result%20Structure%20%28by%20ref%29))
  (Networking|SwitchHasAuthority
    (:Authority
      (bind _asbp_arkde_character (Utilities|Casting|CastToBP_ArkdeCharacter OtherActor))
      (Utilities|IsValid (Class|ArkdeCMCharacter|GetAbilitySystemComponent _asbp_arkde_character)
        (:Is%20Valid
          (GameplayEffects|RemoveActiveGameplayEffectbySourceEffect (Class|ArkdeCMCharacter|GetAbilitySystemComponent _asbp_arkde_character) "/Game/BP/Storm/GE_StormDamage.GE_StormDamage_C" 0 -1))))))

(event OnComponentEndOverlap(Storm)
  (params (OverlappedComponent :type Primitive%20Component%20Object%20Reference) (OtherActor :type Actor%20Object%20Reference) (OtherComp :type Primitive%20Component%20Object%20Reference) (OtherBodyIndex :type Integer))
  (Networking|SwitchHasAuthority
    (:Authority
      (bind _asbp_arkde_character (Utilities|Casting|CastToBP_ArkdeCharacter OtherActor))
      (Utilities|IsValid (Class|ArkdeCMCharacter|GetAbilitySystemComponent _asbp_arkde_character)
        (:Is%20Valid
          (GameplayEffects|ApplyGameplayEffectToSelf :self (Class|ArkdeCMCharacter|GetAbilitySystemComponent _asbp_arkde_character) :GameplayEffectClass "/Game/BP/Storm/GE_StormDamage.GE_StormDamage_C"))))))

(event Custom|resetStormMov
  ;[1 1 1] Storm Movement
  (Utilities|FlowControl|DoOnce false) ; enters at Reset
)

(event Custom|CE_SR_toplayerstart)

(event Custom|resetStormScale
  (Utilities|FlowControl|DoOnce false) ; enters at Reset
)

(event Custom|TimerCountdown1
  (if (> (Variables|Default|GettimeReminingFornextStormToWBP) 0.0)
    (Variables|Default|SettimeReminingFornextStormToWBP (- (Variables|Default|GettimeReminingFornextStormToWBP) 1.0))
    (else
      (Variables|Default|SettimeReminingFornextStormToWBP (Variables|Default|GetTimer))
      (Class|KismetSystemLibrary|PauseTimer 0 "TimerCountdown1")
      (Utilities|FlowControl|Sequence
        (:then_0
          (Utilities|FlowControl|Delay 0.2)
          (Variables|Default|SetReturn%20Value%20Y (.y (Transformation|GetWorldScale (Variables|Default|GetStorm))))
          (Components|Timeline|SetPlayRate (Variables|Default|GetTL_Storm) (/ 1.0 (Variables|Default|GetStormRate)))
          (Utilities|FlowControl|Sequence
            (:then_0
              (Utilities|FlowControl|Delay 0.2)
              (Variables|Default|SetMinScale_0 (- (Variables|Default|GetReturn%20Value%20Y) (Variables|Default|GetMinScale)))
              (if (< (- (Variables|Default|GetReturn%20Value%20Y) (Variables|Default|GetMinScale)) 0.0)
                (Variables|Default|SetMinScale_0 0.0)
                (bind _storm (Timeline|TL_Storm PlayFromStart)
                  (:Update
                    (Variables|Default|SetStorm_0 _storm)
                    (Transformation|SetWorldScale3D (Variables|Default|GetStorm) (Math|Vector|MakeVector (Math|Float|Lerp (Variables|Default|GetMinScale_0) (Variables|Default|GetReturn%20Value%20Y) (Variables|Default|GetStorm_0)) (Math|Float|Lerp (Variables|Default|GetMinScale_0) (Variables|Default|GetReturn%20Value%20Y) (Variables|Default|GetStorm_0)) 7e+02))
                    (bind _output_get (Variables|Default|SetResultScale (Math|Float|Lerp (Variables|Default|GetMinScale_0) (Variables|Default|GetReturn%20Value%20Y) (Variables|Default|GetStorm_0))))
                    (if (== (Math|Float|Truncate _output_get) (Math|Float|Truncate (Variables|Default|GetMinScale_0)))
                      (Variables|Default|SetReturn%20Value%20Y (.y (Transformation|GetWorldScale (Variables|Default|GetStorm))))
                      (Utilities|FlowControl|Sequence
                        (:then_0
                          (Variables|Default|SetStormCirc (+ (Variables|Default|GetStormCirc) 1))
                          (CallFunction|ResetStormScale)
                          (Networking|SwitchHasAuthority
                            (:Authority
                              (if (== (Variables|Default|GetReturn%20Value%20Y) 0.0)
                                (Variables|Default|SettimeReminingFornextStormToWBP 0.0)
                                (else
                                  (Utilities|Time|SetTimerbyFunctionName 0 "TimerCountdown1" 1.0 true))))))
                        (:then_1
                          (Audio|Components|Audio|Stop (Variables|Default|GetTL_Storm)))))))
                (else
                  (Timeline|TL_Storm PlayFromStart))))
            (:then_1
              (Utilities|FlowControl|DoOnce false
                (:Completed
                  (Variables|Default|SetMinScale (Math|Random|RandomFloatinRange (Variables|Default|GetMin) (Variables|Default|GetMax))))))))
        (:then_1
          (Utilities|FlowControl|DoOnce false
            (:Completed
              (Transformation|SetWorldLocation (Variables|Default|GetStorm) (Math|Vector|MakeVector (Math|Random|RandomFloatinRange (Variables|Default|GetMinLocationX) (Variables|Default|GetMaxLocationX)) (Math|Random|RandomFloatinRange (Variables|Default|GetMinLocationY) (Variables|Default|GetMaxLocationY)) 1e+02) false false)
              (Variables|Default|Seton true))))))))

(event EventBeginPlay
  (Networking|SwitchHasAuthority
    (:Authority
      (Utilities|Time|SetTimerbyFunctionName 0 "TimerCountdown1" 1.0 true))))

(fn ConstructionScript)

(fn OnRepon
  (Rendering|SetVisibility (Variables|Default|GetStorm) true true))

(fn OnRepStormCirc)

(fn OnRepMinScale0)

(fn OnRepNewVar0)

(fn OnRepMin)

(fn OnRepMax)

(fn OnRepChangeScaleStorm0
  (bind _output_get (Variables|Default|SetMinScale_0 0.0))
  (Development|PrintString (Utilities|String|ToString(Float) _output_get) true true "(R=0.000000,G=0.660000,B=1.000000,A=1.000000)" 1e+01))

(fn OnRepReturnValueY)

(fn OnRepChangeScaleStorm)

(fn OnRepOff
  (Networking|SwitchHasAuthority))