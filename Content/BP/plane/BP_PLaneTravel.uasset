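; Plane travel actor that places a portal mesh in the level and can respawn a player as a new character.
; On BeginPlay, the server moves the static mesh to a random TargetPoint among all those in the level.
; SpawnPlane destroys the given controller's current pawn, spawns a character at the SpawnTransform location and possesses it.
; Nothing in this Blueprint calls SpawnPlane or links it to the mesh.
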(event Custom|CE_SR_PortalLocation
  (bind _outactors (Actor|GetAllActorsOfClass "/Script/Engine.TargetPoint"))
  (bind _output_get (Variables|Default|SettargetPoint _outactors))
  (Transformation|SetWorldLocationAndRotation (Variables|Default|GetStaticMesh) (Transformation|GetActorLocation (Utilities|Array|Get(acopy) _output_get (Math|Random|RandomIntegerinRange 0 (Utilities|Array|LastIndex _output_get)))) "0, 0, 0" false false))

(event EventBeginPlay
  (Networking|SwitchHasAuthority
    (:Authority
      (CallFunction|CESRPortalLocation))))

(fn ConstructionScript)

(fn SpawnPlane
  (params (Target :type Controller%20Object%20Reference) (SpawnTransform :type Transform))
  (bind _returnvalue (Pawn|GetControlledPawn Target))
  (Utilities|IsValid _returnvalue
    (:Is%20Valid
      (Actor|DestroyActor _returnvalue))
    (:Is%20Not%20Valid
      _))
  (bind _returnvalue_2 (Game|SpawnActorfromClass "/Game/BP/Character/BP_ArkdeCharacter.BP_ArkdeCharacter_C" (Math|Transform|MakeTransform (.location SpawnTransform) "0, 0, 0" "1,1,1") "Undefined" Target 0))
  (Pawn|Possess Target _returnvalue_2))