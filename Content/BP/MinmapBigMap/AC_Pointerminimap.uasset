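; AC_Pointerminimap is a component that registers pointers on the HUD minimap.
; One second after BeginPlay it caches the WBP_HUD reference and calls AddPointerInMyMap with the player character, found through that character's own pointer component rather than this component's owner.
; The readdPointOfEnemy event reuses the cached HUD to register any passed-in actor the same way, via that actor's pointer component.
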(event Custom|readdPointOfEnemy
  (params (actor :type Actor%20Object%20Reference))
  (Utilities|IsValid actor
    (:Is%20Valid
      (Variables|Default|GetAs%20WBP%20HUD
        (:then
          (Default|AddPointerinMyMap (Variables|/Game/BP/WBP/WBP_Stats.WBP_Stats_C|GetWBP_MiniMAp (stale EventBeginPlay _wbp_stats)) (Components|GetOwner (Actor|GetComponentbyClass actor "AC_Pointerminimap_C"))))
        (:else)))))

(event EventBeginPlay
  (Utilities|FlowControl|Delay 1.0)
  (bind _asbp_arkde_character (Utilities|Casting|CastToBP_ArkdeCharacter (Game|GetPlayerCharacter 0)))
  (bind _output_get (Variables|Default|SetAs%20WBP%20HUD (.AsWBP%20HUD (Utilities|Casting|CastToWBP_HUD (HUD|GetHUD (Game|GetPlayerController 0))))))
  (Variables|Default|GetAs%20WBP%20HUD
    (:then
      (bind _wbp_stats (Variables|/Game/BP/core/WBP_HUD.WBP_HUD_C|GetWBP_Stats _output_get)
        (:then
          (Default|AddPointerinMyMap (Variables|/Game/BP/WBP/WBP_Stats.WBP_Stats_C|GetWBP_MiniMAp _wbp_stats) (Components|GetOwner (Actor|GetComponentbyClass _asbp_arkde_character "AC_Pointerminimap_C"))))
        (:else)))
    (:else)))

(event EventTick
  (params (DeltaSeconds :type Float%20%28single-precision%29)))