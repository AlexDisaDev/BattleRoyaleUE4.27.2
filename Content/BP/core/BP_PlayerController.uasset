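; Player controller for a Steam battle royale game, handling the drop-plane intro, lobby hosting and the game-end screen.
; BeginPlay caches the BP_PLaneTravel actor on authority, switches the local view to its camera in the BattleRoyale level, and triggers lobby creation through the Steam game instance.
; Pressing Jump calls the plane's SpawnPlane at its spawn point and disables input.
; GameConclussion replaces all widgets with the win/loss message.
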(event Custom|SetupUI%20Game%20End
  (params (wasSuccesful :type Boolean))
  (Viewport|RemoveAllWidgets)
  (bind _returnvalue (UserInterface|CreateWidget "/Game/BP/WBP/WBP_GameEndMEssage.WBP_GameEndMEssage_C" self))
  (Default|SetupTextGameEnd _returnvalue wasSuccesful)
  (UserInterface|Viewport|AddtoViewport _returnvalue 0))

(event Custom|CE_JumpAirPlane
  (bind _plane (Variables|Default|Getplane))
  (Default|SpawnPlane _plane self (Transformation|GetWorldTransform (Variables|/Game/BP/plane/BP_PLaneTravel.BP_PLaneTravel_C|GetSpawnPoint _plane))))

(event Custom|CE_HostLobby
  (if (Pawn|IsLocalController)
    (bind _asbp_game_instance_steam_advanced (Utilities|Casting|CastToBP_GameInstance_SteamAdvanced (Game|GetGameInstance)))
    (Default|CELobbyCreation _asbp_game_instance_steam_advanced self)))

(event Custom|CustomEvent_0)

(event Custom|CE_PCCamera
  (Game|Player|SetViewTargetwithBlend self (Variables|/Script/Engine.ChildActorComponent|GetChildActor (Variables|/Game/BP/plane/BP_PLaneTravel.BP_PLaneTravel_C|Getcamera1 (Variables|Default|Getplane))) (Variables|Default|GetBlend%20Time) "VTBlend_Linear" 0.0 false))

(event Custom|CE_JumpDisable
  (Variables|Default|SetJump true))

(event EventBeginPlay
  (Utilities|FlowControl|Sequence
    (:then_0
      (Networking|SwitchHasAuthority
        (:Authority
          (bind _returnvalue (Actor|GetActorOfClass "/Game/BP/plane/BP_PLaneTravel.BP_PLaneTravel_C"))
          (Variables|Default|Setplane _returnvalue))))
    (:then_1
      (bind _returnvalue_2 (Game|GetCurrentLevelName true))
      (if (and (Pawn|IsLocalController) (Utilities|Enum|Equal(Enum) _returnvalue_2 "BattleRoyale"))
        (CallFunction|CEPCCamera))
      (Input|EnableInput self))
    (:then_2
      (if (Pawn|IsLocalController)
        (Development|PrintString "Hello")
        (CallFunction|CEHostLobby)))))

(event EventGameConclussion
  (params (WasSuccesful :type Boolean))
  (CallFunction|SetupUIGameEnd WasSuccesful))

(event Input|ActionEvents|InputActionJump
  (params (Key :type Key%20Structure :default "None"))
  (:Pressed
    (CallFunction|CEJumpAirPlane)
    (Input|DisableInput self)))

(fn ConstructionScript)

(fn PCOwner
  (return self))

(fn PcOwner
  (return self))