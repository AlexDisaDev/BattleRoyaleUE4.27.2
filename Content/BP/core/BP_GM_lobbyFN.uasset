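; Lobby game mode that seats each connected player on a platform spawner with a spawned character.
; At BeginPlay it collects BP_platformSpawner actors, ordered by index tags.
; Login (which also runs ToggleSpeaking for voice) and logout update the controller list, wait via a delay-polling macro for setup, then fill free platforms and clear departed players' ones.
; SetupPlatform and UpdatePlayersOnPLatform functions are unused variants of the custom events.
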(event Custom|CE_SetupPlatform
  (bind _outactors (Actor|GetAllActorsOfClass "/Game/BP/Lobby/BP_platformSpawner.BP_platformSpawner_C"))
  (for _index (range 0 (Utilities|Array|LastIndex _outactors))
    (bind _outactors_2 (Actor|GetAllActorsOfClasswithTag "/Game/BP/Lobby/BP_platformSpawner.BP_platformSpawner_C" (Utilities|String|StringToName (Utilities|String|ToString(Integer) _index))))
    (Utilities|Array|Add (Variables|Default|GetPlayerPlatforms) (Utilities|Array|Get(acopy) _outactors_2)))
  (Variables|Default|SetbSetupPlatformDone true))

(event Custom|CE_UpdatePlatform
  ;[1 1 1] pc already added
  (bind _array_element (Utilities|Array|ForEachLoopwithBreak (Variables|Default|GetPCs))
    (:LoopBody
      (Variables|Default|SetLoop_PCAlreadyAdded false)
      (bind _array_element_2 (Utilities|Array|ForEachLoopwithBreak (Variables|Default|GetPlayerPlatforms) :!label _label)
        (:LoopBody
          (if (== (Variables|/Game/BP/Lobby/BP_platformSpawner.BP_platformSpawner_C|GetPC _array_element_2) _array_element)
            (Variables|Default|SetLoop_PCAlreadyAdded true)
            (goto _label Break)))
        (:Completed
          (if (not (Variables|Default|GetLoop_PCAlreadyAdded))
            (bind _array_element_3 (Utilities|Array|ForEachLoopwithBreak (Variables|Default|GetPlayerPlatforms) :!label _label_2)
              (:LoopBody
                (Utilities|IsValid (Variables|/Game/BP/Lobby/BP_platformSpawner.BP_platformSpawner_C|GetPC _array_element_3)
                  (:Is%20Not%20Valid
                    (Default|CESpawnCharacter _array_element_3 _array_element)
                    (goto _label_2 Break)))))))))
    (:Completed
      ;[1 1 1] remove players from platform
      (bind _array_element_4 (Utilities|Array|ForEachLoopwithBreak (Variables|Default|GetPlayerPlatforms))
        (:LoopBody
          (if (not (Utilities|Array|ContainsItem (Variables|Default|GetPCs) (Variables|/Game/BP/Lobby/BP_platformSpawner.BP_platformSpawner_C|GetPC _array_element_4)))
            (Default|CEClearPlatform _array_element_4)))))))

(event EventBeginPlay
  (CallFunction|CESetupPlatform))

(event EventTick
  (params (DeltaSeconds :type Float%20%28single-precision%29)))

(event EventPostLogin
  (params (NewPlayer :type Player%20Controller%20Object%20Reference))
  (Utilities|Array|Add (Variables|Default|GetPCs) NewPlayer)
  (Development|ExecuteConsoleCommand "ToggleSpeaking 1" NewPlayer)
  (Utilities|IfPlatformSetupDone
    (:true
      (CallFunction|CEUpdatePlatform))))

(event EventOnLogout
  (params (ExitingController :type Controller%20Object%20Reference))
  (bind _asplayer_controller (Utilities|Casting|CastToPlayerController ExitingController))
  (Utilities|Array|RemoveItem (Variables|Default|GetPCs) _asplayer_controller)
  (Utilities|IfPlatformSetupDone
    (:true
      (CallFunction|CEUpdatePlatform))))

(fn ConstructionScript)

(fn SetupPlatform
  (bind _outactors (Actor|GetAllActorsOfClass "/Game/BP/Lobby/BP_platformSpawner.BP_platformSpawner_C"))
  (for _index (range 0 (Utilities|Array|LastIndex _outactors))
    (bind _outactors_2 (Actor|GetAllActorsOfClasswithTag "/Game/BP/Lobby/BP_platformSpawner.BP_platformSpawner_C" (Utilities|String|StringToName (Utilities|String|ToString(Integer) _index))))
    (Utilities|Array|Add (Variables|Default|GetPlayerPlatforms) (Utilities|Array|Get(acopy) _outactors_2)))
  (Variables|Default|SetbSetupPlatformDone true))

(fn UpdatePlayersonPLatform
  ;[1 1 1] pc already added
  (bind _array_element (Utilities|Array|ForEachLoopwithBreak (Variables|Default|GetPCs))
    (:LoopBody
      (LocalVariables|SetLoop_PCAlreadyAdded false)
      (bind _array_element_2 (Utilities|Array|ForEachLoopwithBreak (Variables|Default|GetPlayerPlatforms) :!label _label)
        (:LoopBody
          (if (== (Variables|/Game/BP/Lobby/BP_platformSpawner.BP_platformSpawner_C|GetPC _array_element_2) _array_element)
            (LocalVariables|SetLoop_PCAlreadyAdded true)
            (goto _label Break)))
        (:Completed
          (if (not (LocalVariables|GetLoop_PCAlreadyAdded))
            (bind _array_element_3 (Utilities|Array|ForEachLoopwithBreak (Variables|Default|GetPlayerPlatforms))
              (:LoopBody
                (Utilities|IsValid (Variables|/Game/BP/Lobby/BP_platformSpawner.BP_platformSpawner_C|GetPC _array_element_3)
                  (:Is%20Not%20Valid
                    (Default|CESpawnCharacter _array_element_3 _array_element)))))))))
    (:Completed
      ;[1 1 1] remove players from platform
      (bind _array_element_4 (Utilities|Array|ForEachLoopwithBreak (Variables|Default|GetPlayerPlatforms))
        (:LoopBody
          (if (Utilities|Array|ContainsItem (Variables|Default|GetPCs) (Variables|/Game/BP/Lobby/BP_platformSpawner.BP_platformSpawner_C|GetPC _array_element_4))
            (Default|CEClearPlatform _array_element_4)))))))