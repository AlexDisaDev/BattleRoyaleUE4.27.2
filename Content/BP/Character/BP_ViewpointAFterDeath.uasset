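; BP_ViewpointAFterDeath is, by its name, a post-death viewpoint meant to trail a surviving BP_ArkdeCharacter at an X offset.
; The foundActor event picks the first valid entry in AllActorInGame as the target.
; The swept follow move, its retargeting fallback and the gathering of characters are all disconnected from events.
; BeginPlay and Tick are empty, so the viewpoint does nothing by itself.
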(event Custom|foundActor
  (bind _array_element (Utilities|Array|ForEachLoopwithBreak (Variables|Default|GetAllActorInGame) :!label _label)
    (:LoopBody
      (Utilities|IsValid _array_element
        (:Is%20Valid
          (goto _label Break))))
    (:Completed
      (Variables|Default|Setactor _array_element))))

(event EventBeginPlay)

(event EventTick
  (params (DeltaSeconds :type Float%20%28single-precision%29)))

(fn ConstructionScript)